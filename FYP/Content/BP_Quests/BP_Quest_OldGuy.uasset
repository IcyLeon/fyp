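; Quest Blueprint for the Old Guy quest, where Henry, the ghostly storyteller, receives photos from the player.
; Tick polls NPC dialogue state to swap dialogue lists, open drag-and-drop submission, handle failed attempts and advance objectives.
; It also grades camera photo-composition challenges for hidden objectives, triggering feedback and Vessel follow-up dialogue.
; Picture pickups are shown or hidden with quest state, and submission progress feeds the quest UI.
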(event Custom|SetVisibleQuestItems
  (bind _questref (CallFunction|GetMainQuest))
  (bind _outactors (Actor|GetAllActorsOfClass "/Game/Archery/PicturePickup.PicturePickup_C"))
  (if (not (.Status (Utilities|Struct|BreakQuestInfo _questref)))
    (if (.StartQuest? (Utilities|Struct|BreakQuestInfo _questref))
      (for _array_element _outactors
        (Rendering|SetActorHiddenInGame _array_element false)
        (Collision|SetActorEnableCollision _array_element true)
        (if (Variables|/Game/Archery/PickUps.PickUps_C|GetEnableGravity _array_element)
          (Physics|SetSimulatePhysics (Variables|/Game/Archery/PickUps.PickUps_C|GetCube _array_element) true)))
      (else
        (for _array_element_2 _outactors
          (Rendering|SetActorHiddenInGame _array_element_2 true)
          (Collision|SetActorEnableCollision _array_element_2 false)
          (if (Variables|/Game/Archery/PickUps.PickUps_C|GetEnableGravity _array_element_2)
            (Physics|SetSimulatePhysics (Variables|/Game/Archery/PickUps.PickUps_C|GetCube _array_element_2) false)
            (Transformation|SetActorLocation _array_element_2 (Transformation|GetWorldLocation (Variables|/Game/Archery/PickUps.PickUps_C|GetCube _array_element_2)) false false)))))))

(event Custom|TakePhotoDialogue
  (bind _player (Variables|Default|GetPlayer))
  (bind _questlogmanager (Variables|/Game/ThirdPerson/Blueprints/BP_ThirdPersonCharacter.BP_ThirdPersonCharacter_C|GetQuestLogManager _player))
  (bind _currentgadget (Variables|/Game/ThirdPerson/Blueprints/BP_ThirdPersonCharacter.BP_ThirdPersonCharacter_C|GetCurrentGadget _player))
  (bind _currenttrackquest (Variables|/Game/Data/QuestLogManager.QuestLogManager_C|GetCurrentTrackQuest _questlogmanager))
  (bind _currenttrackquest_2 (Variables|/Game/Data/QuestLogManager.QuestLogManager_C|GetCurrentTrackQuest _questlogmanager))
  (bind _output (Utilities|Array|Get(acopy) (.hiddenobjectives _currenttrackquest) (.currenthiddenobjectiveidx _currenttrackquest)))
  (bind (_objectivedesc _objectivelocation _complete_ _desiredamount _showprogress_ _target _questtype) (Utilities|Struct|BreakObjectives _output))
  (Utilities|IsValid _player
    (:Is%20Valid
      (if (Utilities|Enum|Equal(Enum) (.questid _currenttrackquest_2) (Variables|Default|GetQuestRow))
        (Utilities|IsValid _currentgadget
          (:Is%20Valid
            (bind _ascamera (Utilities|Casting|CastToCamera _currentgadget))
            (bind _cameraframe (Variables|/Game/Archery/Camera.Camera_C|GetCameraFrame _ascamera)
              (:then
                (Default|CallSendCameraREF _cameraframe self (Utilities|Array|Get(acopy) (.hiddenobjectives _currenttrackquest_2) (.currenthiddenobjectiveidx _currenttrackquest_2))))
              (:else
                _))
            (bind _take_photo_ui (Variables|/Game/Archery/Camera.Camera_C|GetTake%20Photo%20UI _ascamera)
              (:then
                (if (Math|Boolean|ANDBoolean (not _complete_) (Utilities|Enum|Equal(Enum) _questtype "NewEnumerator6") (Variables|/Game/Data/PhotoManager.PhotoManager_C|GetSuccess? (Variables|/Game/Actors/GameManager.GameManager_C|GetPhotoManager (Variables|Default|GetGameManager))))
                  (switch int (.currenthiddenobjectiveidx _currenttrackquest)
                    (:1
                      (Variables|Default|SetDialoguesList (Variables|Default|GetSuccessMazeTakePhotoDialogue))
                      (CallFunction|PhotoMessageOutcome "Correct application of Foreshadowing Interest"))
                    (:3
                      (Variables|Default|SetDialoguesList (Variables|Default|GetSuccessGardenTakePhotoDialogue))
                      (CallFunction|PhotoMessageOutcome "Correct application of Rule of Third")))
                  (Default|UpdateHiddenQuestObjectives (Variables|Default|GetAs%20BP%20Game%20Instance) (Variables|Default|GetQuestRow) "NewEnumerator6" (.currenthiddenobjectiveidx _currenttrackquest))
                  (else
                    (switch int (.currenthiddenobjectiveidx _currenttrackquest)
                      (:1
                        (Variables|Default|SetDialoguesList (Variables|Default|GetFailMazeTakePhotoDialogue))
                        (CallFunction|PhotoMessageOutcome "Wrong, Try again?"))
                      (:3
                        (Variables|Default|SetDialoguesList (Variables|Default|GetFailGardenTakePhotoDialogue))
                        (CallFunction|PhotoMessageOutcome "Wrong, Try again?")))))
                (EventDispatchers|BindEventtoDeleteCamera _take_photo_ui (delegate Custom|CustomEvent)))
              (:else
                (Variables|Default|SetSpawnMsg? true)))))))))

(event Custom|UpdateInteractions
  (bind _midinteractiondialogues (Variables|Default|GetMidInteractionDialogues))
  (bind _gamemanager (Variables|Default|GetGameManager))
  (bind _givingitems (Variables|Default|GetGivingItems))
  (bind _actorref (Variables|Default|GetActorREF))
  (bind _npcmanager (Variables|/Game/Actors/GameManager.GameManager_C|GetNPCManager _gamemanager))
  (bind _questref (Default|GetQuest (Variables|Default|GetAs%20BP%20Game%20Instance) (Variables|Default|GetQuestRow)))
  (if (Utilities|DoesObjectImplementInterface _actorref "/Game/Interfaces/InteractDialogues.InteractDialogues_C")
    (bind _getstate (Class|InteractDialogues|InteractDialogues(Message) _actorref "NewEnumerator3"))
    (switch Utilities|FlowControl|Switch|SwitchonNPCStates _getstate
      (:NewEnumerator1
        (if (and (Utilities|Array|Identical (Variables|Default|GetDialoguesList) (Variables|Default|GetStartQuestDialogueList)) (not (.StartQuest? (Utilities|Struct|BreakQuestInfo _questref))))
          (if (and (== (Variables|/Game/Data/NPCManager.NPCManager_C|GetCurrentDialogueIdx _npcmanager) 1) (== (Variables|/Game/Data/NPCManager.NPCManager_C|GetCurrentDIalogueTalkingIdx _npcmanager) 0))
            (Class|NPCNames|NPCNames(Message) (Variables|Default|GetActorREF) "Henry" "Ghostly Storyteller" true))))
      (:NewEnumerator2
        (if (Utilities|Array|Identical (Variables|Default|GetDialoguesList) (Variables|Default|GetFinishQuestDialogue))
          (Default|UpdateQuestObjectives (Variables|Default|GetAs%20BP%20Game%20Instance) (Variables|Default|GetQuestRow) "NewEnumerator2" 3))
        (if (.Complete? (Utilities|Struct|BreakObjectives (Utilities|Array|Get(acopy) (.Objectives (Utilities|Struct|BreakQuestInfo _questref)) 3)))
          (Variables|Default|SetDialoguesList (Variables|Default|GetPostQuestDialogue))
          (Class|InteractDialogues|InteractDialogues(Message) (Variables|Default|GetActorREF) "NewEnumerator0" :!label _label)
          (Variables|/Game/ThirdPerson/Blueprints/BP_ThirdPersonCharacter.BP_ThirdPersonCharacter_C|SetisInteracting (Variables|Default|GetPlayer) false)
          (elif (not (.StartQuest? (Utilities|Struct|BreakQuestInfo _questref)))
            (Variables|Default|SetDialoguesList _midinteractiondialogues)
            (CallFunction|ResetCameraPan)
            (goto _label)
            (else
              (Variables|Default|SetDialoguesList _midinteractiondialogues)
              (if (Math|Boolean|ANDBoolean (== (Variables|/Game/Data/NPCManager.NPCManager_C|GetPrevChoiceNo (Variables|/Game/Actors/GameManager.GameManager_C|GetNPCManager (Variables|Default|GetGameManager))) 0) (Utilities|Array|Identical _midinteractiondialogues (Variables|Default|GetDialoguesList)) (== (Variables|/Game/ThirdPerson/Blueprints/BP_ThirdPersonCharacter.BP_ThirdPersonCharacter_C|GetLock%20Closest%20NPC (Variables|Default|GetPlayer)) (Variables|Default|GetActorREF)))
                (Default|OpenDragandDropUI _givingitems)
                (Variables|/Game/Widget/DragAndDropUI.DragAndDropUI_C|SetSubmitOthers? (Variables|/Game/Data/GivingItems.GivingItems_C|GetDragAndDropUI _givingitems) true)
                (EventDispatchers|BindEventtoCallClosingButton _givingitems (delegate Custom|CustomEvent_0))
                (else
                  (goto _label))))))))))

(event Custom|CustomEvent_0
  (params (CloseBtnClick? :type Boolean) (AllCorrect? :type Boolean))
  (bind _actorref (Variables|Default|GetActorREF))
  (bind _attempts (Variables|Default|GetAttempts))
  (if CloseBtnClick?
    (Class|InteractDialogues|InteractDialogues(Message) (Variables|Default|GetActorREF) "NewEnumerator0")
    (Variables|/Game/ThirdPerson/Blueprints/BP_ThirdPersonCharacter.BP_ThirdPersonCharacter_C|SetisInteracting (Variables|Default|GetPlayer) false)
    (else
      (if AllCorrect?
        (bind _complete_ (Default|GiveItemSuccess (Variables|Default|GetGivingItems) AllCorrect?))
        (if _complete_
          (Variables|Default|SetDialoguesList (Variables|Default|GetFinishQuestDialogue))
          (else
            (switch int (Variables|/Game/Data/GivingItems.GivingItems_C|GetCount%20Item%20Give (Variables|Default|GetGivingItems))
              (:1
                (Variables|Default|SetDialoguesList (Variables|Default|GetFirstSubmissionDialogues))
                (Variables|Default|SetFinishGivingFIrstPhoto true))
              (:2
                (Variables|Default|SetDialoguesList (Variables|Default|GetSecondSubmissionDialogue))))))
        (else
          (if (>= _attempts 3)
            (Variables|Default|SetDialoguesList (Variables|Default|GetThreeAttemptFailedDialogue))
            (else
              (Variables|Default|SetDialoguesList (Variables|Default|GetFailedDialogue))))
          (Math|Integer|IncrementInt _attempts
            (:%20%20
              _))))
      (Class|InteractDialogues|InteractDialogues(Message) _actorref "NewEnumerator0")
      (Class|Interactable|Interact(Message) _actorref (Variables|Default|GetPlayer)))))

(event Custom|CustomEvent_1
  (bind _player (Variables|Default|GetPlayer))
  (bind _dialoguehandler (Variables|/Game/ThirdPerson/Blueprints/BP_ThirdPersonCharacter.BP_ThirdPersonCharacter_C|GetDialogueHandler _player))
  (Utilities|IsValid (Variables|/Game/Data/DialogueHandler.DialogueHandler_C|GetDialogueUI _dialoguehandler)
    (:Is%20Not%20Valid
      (if (Utilities|Array|Identical (Variables|Default|GetDialoguesList) (Variables|Default|GetSuccessGardenTakePhotoDialogue))
        (bind _returnvalue (Actor|GetActorOfClass "/Game/Vessel/Vessel.Vessel_C"))
        (Utilities|IsValid _returnvalue
          (:Is%20Valid
            (Default|GenerateDialogue _dialoguehandler (Variables|/Game/Vessel/Vessel.Vessel_C|GetSuccessGardenPhoto _returnvalue) (Variables|Default|GetPlayer) false true _returnvalue true (Variables|Default|GetQuestRow))
            (Utilities|Time|ClearandInvalidateTimerbyHandle (stale Custom|CustomEvent _returnvalue))))))))

(event Custom|CustomEvent
  (bind _player (Variables|Default|GetPlayer))
  (bind _dialogueslist (Variables|Default|GetDialoguesList))
  (bind _player_2 (Variables|Default|GetPlayer))
  (bind _actorref (Variables|Default|GetActorREF))
  (bind _player_3 (Variables|Default|GetPlayer))
  (bind _questlogmanager (Variables|/Game/ThirdPerson/Blueprints/BP_ThirdPersonCharacter.BP_ThirdPersonCharacter_C|GetQuestLogManager _player))
  (bind _dialoguehandler (Variables|/Game/ThirdPerson/Blueprints/BP_ThirdPersonCharacter.BP_ThirdPersonCharacter_C|GetDialogueHandler _player_3))
  (bind _currenttrackquest (Variables|/Game/Data/QuestLogManager.QuestLogManager_C|GetCurrentTrackQuest _questlogmanager))
  (bind _dialogueui (Variables|/Game/Data/DialogueHandler.DialogueHandler_C|GetDialogueUI _dialoguehandler))
  (bind _output (Utilities|Array|Get(acopy) (.hiddenobjectives _currenttrackquest) (.currenthiddenobjectiveidx _currenttrackquest)))
  (bind (_objectivedesc _objectivelocation _complete_ _desiredamount _showprogress_ _target _questtype) (Utilities|Struct|BreakObjectives _output))
  (Utilities|IsValid _dialogueui
    (:Is%20Valid
      (Default|ForceStop _dialogueui))
    (:Is%20Not%20Valid
      _))
  (if (Math|Boolean|ANDBoolean (not _complete_) (Utilities|Enum|Equal(Enum) _questtype "NewEnumerator6") (Variables|/Game/Data/PhotoManager.PhotoManager_C|GetSuccess? (Variables|/Game/Actors/GameManager.GameManager_C|GetPhotoManager (Variables|Default|GetGameManager))))
    (Default|GenerateDialogue _dialoguehandler _dialogueslist _player_2 false true _actorref true (Variables|Default|GetQuestRow))
    (else
      (Default|GenerateDialogue _dialoguehandler _dialogueslist _player_2 false true _actorref true "NewEnumerator2")))
  (bind _returnvalue (Utilities|Time|SetTimerbyEvent (delegate Custom|CustomEvent_1) 0.01 true)))

(event Custom|MobiroRelicTalk
  (bind _player (Variables|Default|GetPlayer))
  (bind _dialoguehandler (Variables|/Game/ThirdPerson/Blueprints/BP_ThirdPersonCharacter.BP_ThirdPersonCharacter_C|GetDialogueHandler _player))
  (bind _questref (Default|GetQuest (Variables|Default|GetAs%20BP%20Game%20Instance) (Variables|Default|GetQuestRow)))
  (if (and (.Complete? (Utilities|Struct|BreakObjectives (Utilities|Array|Get(acopy) (.Objectives (Utilities|Struct|BreakQuestInfo _questref)) 4))) (not (Variables|Default|GetFinishMobiroRelic?)))
    (Utilities|IsValid (Variables|/Game/Data/DialogueHandler.DialogueHandler_C|GetDialogueUI _dialoguehandler)
      (:Is%20Not%20Valid
        (bind _returnvalue (Actor|GetActorOfClass "/Game/Vessel/Vessel.Vessel_C"))
        (Utilities|IsValid _returnvalue
          (:Is%20Valid
            (Default|GenerateDialogue _dialoguehandler (Variables|/Game/Vessel/Vessel.Vessel_C|GetMobiroRelic _returnvalue) (Variables|Default|GetPlayer) false true _returnvalue true (Variables|Default|GetQuestRow))
            (Variables|Default|SetFinishMobiroRelic? true)))))))

(event Custom|GiveBacktoHenryObjective
  (bind _actorref (Variables|Default|GetActorREF))
  (if (Variables|Default|GetFinishGivingFIrstPhoto)
    (if (Utilities|DoesObjectImplementInterface _actorref "/Game/Interfaces/InteractDialogues.InteractDialogues_C")
      (bind _getstate (Class|InteractDialogues|InteractDialogues(Message) _actorref "NewEnumerator3"))
      (switch Utilities|FlowControl|Switch|SwitchonNPCStates _getstate
        (:NewEnumerator0
          _)
        (:NewEnumerator2
          _))
      (Default|UpdateQuestObjectives (Variables|Default|GetAs%20BP%20Game%20Instance) (Variables|Default|GetQuestRow) "NewEnumerator2" 2))))

(event Custom|ResetCameraPan
  (Variables|/Game/Data/GivingItems.GivingItems_C|SetPlayer (Variables|Default|GetGivingItems) (Variables|Default|GetPlayer))
  (bind _outactors (Actor|GetAllActorsOfClass "/Game/Actors/CameraPan.CameraPan_C"))
  (for _array_element _outactors
    (Variables|/Game/Actors/CameraPan.CameraPan_C|SetFirstEncounter? _array_element true)))

(event EventBeginPlay
  (|CallParentFunction)
  (Variables|Default|SetDialoguesList (Variables|Default|GetStartQuestDialogueList)))

(event Collision|EventActorBeginOverlap
  (params (OtherActor :type Actor%20Object%20Reference))
  (|CallParentFunction OtherActor) ; This node is disabled and will not be called.\nDrag off pins to build functionality.
)

(event EventTick
  (params (DeltaSeconds :type Float%20%28single-precision%29))
  (|CallParentFunction DeltaSeconds)
  (CallFunction|UpdateInteractions)
  (CallFunction|CheckEquipItemObjective "NewEnumerator10")
  (CallFunction|CheckIteminInv "NewEnumerator3")
  (CallFunction|GiveBacktoHenryObjective)
  (CallFunction|MobiroRelicTalk)
  (CallFunction|TakePhotoDialogue)
  (CallFunction|SetVisibleQuestItems))

(fn ConstructionScript
  (|CallParentFunction))

(fn SendMapDetails
  (bind (_world_position _widget _worldmapiconsize _iconsinfo _texture _actorref _minimapwidget _minimapiconsize _visible_) (|CallParentFunction))
  (return _world_position _widget _worldmapiconsize _iconsinfo _texture _actorref _minimapwidget _minimapiconsize _visible_))

(fn GetMainQuest
  (bind (_questname _questref) (|CallParentFunction))
  (return _questname _questref))

(fn GetQuestObjective
  (bind _currentquesttrack (Variables|/Game/Widget/QuestUI.QuestUI_C|GetCurrentQuestTrack (Variables|/Game/ThirdPerson/Blueprints/BP_ThirdPersonCharacter.BP_ThirdPersonCharacter_C|GetQuestUI (Variables|Default|GetPlayer)))
    (:then
      (switch Utilities|FlowControl|Switch|SwitchonQuestRow (.QuestID (Utilities|Struct|BreakQuestInfo (Variables|/Game/Widget/QuestButton.QuestButton_C|GetQuestInfoREF _currentquesttrack)))
        (:NewEnumerator0
          (switch int (.CurrentObjectiveIdx (Utilities|Struct|BreakQuestInfo (Variables|/Game/Widget/QuestButton.QuestButton_C|GetQuestInfoREF _currentquesttrack)))
            (:0
              _)
            (:1
              _)
            (:2
              (Variables|Default|SetObjective%20ID (.CurrentObjectiveIdx (Utilities|Struct|BreakQuestInfo (Variables|/Game/Widget/QuestButton.QuestButton_C|GetQuestInfoREF _currentquesttrack))) :!label _label))
            (:3
              (goto _label))
            (:5
              (goto _label))))
        (:NewEnumerator1
          (switch int (.CurrentObjectiveIdx (Utilities|Struct|BreakQuestInfo (Variables|/Game/Widget/QuestButton.QuestButton_C|GetQuestInfoREF _currentquesttrack)))
            (:2
              (goto _label)))))
      (return (Utilities|Array|Get(acopy) (.Objectives (Utilities|Struct|BreakQuestInfo (Variables|/Game/Widget/QuestButton.QuestButton_C|GetQuestInfoREF _currentquesttrack))) (Variables|Default|GetObjective%20ID)) (Variables|Default|GetObjective%20ID) (Variables|/Game/Widget/QuestButton.QuestButton_C|GetQuestInfoREF _currentquesttrack)))
    (:else)))

(fn SendProgress
  (bind _givingitems (Variables|Default|GetGivingItems))
  (bind _givingitems_2 (Variables|Default|GetGivingItems))
  (bind _player (Variables|Default|GetPlayer))
  (bind _questui (Variables|/Game/ThirdPerson/Blueprints/BP_ThirdPersonCharacter.BP_ThirdPersonCharacter_C|GetQuestUI _player))
  (bind _itemstobegivenaway (Variables|/Game/Data/GivingItems.GivingItems_C|GetItemsToBeGivenAway _givingitems))
  (bind _count_item_give (Variables|/Game/Data/GivingItems.GivingItems_C|GetCount%20Item%20Give _givingitems_2))
  (bind _returnvalue (Utilities|Array|Length _itemstobegivenaway))
  (Utilities|IsValid _questui
    (:Is%20Valid
      (bind _quest_button_ref (Default|FindQuestButton _questui (Variables|Default|GetQuestRow)))
      (Utilities|IsValid _quest_button_ref
        (:Is%20Valid
          (return _quest_button_ref (Math|Conversions|ToFloat(Integer) _count_item_give) (Math|Conversions|ToFloat(Integer) _returnvalue) (Utilities|String|Append (Utilities|String|ToString(Integer) _count_item_give) "/" (Utilities|String|ToString(Integer) _returnvalue) " Photos Submitted")))))))