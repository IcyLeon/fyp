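; Exploration quest actor, a child Blueprint that automatically starts its quest once the tutorial manager leaves its first state.
; Tick polls the game instance for the quest row and, if it is unstarted, starts it and sets the parent-provided main quest as the quest log's tracked quest.
; Its map details return zeroed and hidden, so it supplies no visible map marker.
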(event EventBeginPlay
  (|CallParentFunction))

(event Collision|EventActorBeginOverlap
  (params (OtherActor :type Actor%20Object%20Reference))
  (|CallParentFunction OtherActor) ; This node is disabled and will not be called.\nDrag off pins to build functionality.
)

(event EventTick
  (params (DeltaSeconds :type Float%20%28single-precision%29))
  (bind _as_bp_game_instance (Variables|Default|GetAs%20BP%20Game%20Instance))
  (|CallParentFunction DeltaSeconds)
  (bind _questref (Default|GetQuest _as_bp_game_instance (Variables|Default|GetQuestRow)))
  (if (and (not (.StartQuest? (Utilities|Struct|BreakQuestInfo _questref))) (Utilities|Enum|NotEqual(Enum) (Variables|/Game/Data/TutorialManager.TutorialManager_C|GetTutorialState (Variables|/Game/Actors/GameManager.GameManager_C|GetTutorialManager (Variables|Default|GetGameManager))) "NewEnumerator0"))
    (Default|StartQuest _as_bp_game_instance (Variables|Default|GetQuestRow))
    (bind _questref_2 (CallFunction|GetMainQuest))
    (Variables|/Game/Data/QuestLogManager.QuestLogManager_C|SetCurrentTrackQuest (Variables|/Game/ThirdPerson/Blueprints/BP_ThirdPersonCharacter.BP_ThirdPersonCharacter_C|GetQuestLogManager (Variables|Default|GetPlayer)) _questref_2)))

(fn ConstructionScript
  (|CallParentFunction))

(fn GetMainQuest
  (bind (_questname _questref) (|CallParentFunction))
  (return _questname _questref))

(fn SendMapDetails
  (return "0, 0, 0" 0 "" "" 0 0 0 "" false))