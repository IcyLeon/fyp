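; BP_Quest is a quest actor that tracks one quest row's current objective and supplies its map and minimap marker.
; It reads quest state from BP_GameInstance and matches the player's locked NPC class against the objective target.
; Dialogue objectives are polled on Tick, while interact and equip events also report to the player's QuestLogManager.
; SendMapDetails creates icon widgets and hides the question-mark marker once the quest's Status is true.
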(event Custom|InteractionsDialogueObjective
  (bind _player (Variables|Default|GetPlayer))
  (bind _lock_closest_npc (Variables|/Game/ThirdPerson/Blueprints/BP_ThirdPersonCharacter.BP_ThirdPersonCharacter_C|GetLock%20Closest%20NPC _player))
  (Utilities|IsValid _player
    (:Is%20Valid
      (Utilities|IsValid _lock_closest_npc
        (:Is%20Valid
          (if (Utilities|DoesObjectImplementInterface _lock_closest_npc "/Game/Interfaces/Interactable.Interactable_C")
            (bind _questref (Default|GetQuest (Variables|Default|GetAs%20BP%20Game%20Instance) (Variables|Default|GetQuestRow)))
            (if (and (not (.Status (Utilities|Struct|BreakQuestInfo _questref))) (.StartQuest? (Utilities|Struct|BreakQuestInfo _questref)))
              (if (== (Utilities|GetClass _lock_closest_npc) (.Target (Utilities|Struct|BreakObjectives (Utilities|Array|Get(acopy) (.Objectives (Utilities|Struct|BreakQuestInfo _questref)) (.CurrentObjectiveIdx (Utilities|Struct|BreakQuestInfo _questref))))))
                (if (Utilities|DoesObjectImplementInterface _lock_closest_npc "/Game/Interfaces/InteractDialogues.InteractDialogues_C")
                  (bind _getstate (Class|InteractDialogues|InteractDialogues(Message) _lock_closest_npc "NewEnumerator3"))
                  (if (and (Utilities|Enum|Equal(Enum) _getstate "NewEnumerator2") (Variables|/Game/ThirdPerson/Blueprints/BP_ThirdPersonCharacter.BP_ThirdPersonCharacter_C|GetisInteracting (Variables|Default|GetPlayer)))
                    (Default|CallInteractDialogues (Variables|/Game/ThirdPerson/Blueprints/BP_ThirdPersonCharacter.BP_ThirdPersonCharacter_C|GetQuestLogManager (Variables|Default|GetPlayer)) self)))))))))))

(event Custom|InteractObjective
  (bind _player (Variables|Default|GetPlayer))
  (bind _lock_closest_npc (Variables|/Game/ThirdPerson/Blueprints/BP_ThirdPersonCharacter.BP_ThirdPersonCharacter_C|GetLock%20Closest%20NPC _player))
  (Utilities|IsValid _player
    (:Is%20Valid
      (Utilities|IsValid _lock_closest_npc
        (:Is%20Valid
          (if (Utilities|DoesObjectImplementInterface _lock_closest_npc "/Game/Interfaces/Interactable.Interactable_C")
            (bind _questref (Default|GetQuest (Variables|Default|GetAs%20BP%20Game%20Instance) (Variables|Default|GetQuestRow)))
            (if (and (not (.Status (Utilities|Struct|BreakQuestInfo _questref))) (.StartQuest? (Utilities|Struct|BreakQuestInfo _questref)))
              (if (== (Utilities|GetClass _lock_closest_npc) (.Target (Utilities|Struct|BreakObjectives (Utilities|Array|Get(acopy) (.Objectives (Utilities|Struct|BreakQuestInfo _questref)) (.CurrentObjectiveIdx (Utilities|Struct|BreakQuestInfo _questref))))))
                (Default|CallInteracted (Variables|/Game/ThirdPerson/Blueprints/BP_ThirdPersonCharacter.BP_ThirdPersonCharacter_C|GetQuestLogManager (Variables|Default|GetPlayer)) self)))))))))

(event Custom|CheckEquipItemObjective
  (params (Item :type ItemRow%20Enum :default "NewEnumerator3"))
  (Default|CallEquip (Variables|/Game/ThirdPerson/Blueprints/BP_ThirdPersonCharacter.BP_ThirdPersonCharacter_C|GetQuestLogManager (Variables|Default|GetPlayer)) Item self))

(event EventBeginPlay
  (bind _asbp_game_instance (Utilities|Casting|CastToBP_GameInstance (Game|GetGameInstance)))
  (Variables|Default|SetAs%20BP%20Game%20Instance _asbp_game_instance)
  (Variables|Default|SetActorREF (Actor|GetAttachParentActor))
  (bind _asbp_third_person_character (Utilities|Casting|CastToBP_ThirdPersonCharacter (Game|GetPlayerCharacter 0)))
  (Variables|Default|SetPlayer _asbp_third_person_character)
  (bind _returnvalue (Actor|GetActorOfClass "/Game/Actors/GameManager.GameManager_C"))
  (Variables|Default|SetGameManager _returnvalue))

(event Collision|EventActorBeginOverlap
  (params (OtherActor :type Actor%20Object%20Reference)))

(event EventTick
  (params (DeltaSeconds :type Float%20%28single-precision%29))
  (CallFunction|InteractionsDialogueObjective))

(fn ConstructionScript)

(fn GetMainQuest
  (bind _questrow (Variables|Default|GetQuestRow))
  (bind _questref (Default|GetQuest (Variables|Default|GetAs%20BP%20Game%20Instance) _questrow))
  (return _questrow _questref))

(fn SendMapDetails
  (bind _returnvalue (Transformation|GetActorLocation))
  (bind _self self)
  (Utilities|IsValid (Variables|Default|GetIcon)
    (:Is%20Valid
      (bind _givebacksize (Class|SendMapSize|SendMapSIze(Message) (Variables|Default|GetIcon) "(X=25.000000,Y=40.000000)"))
      (bind _givebacksize_2 (Class|SendMapSize|SendMapSIze(Message) (Variables|Default|GetMinimap%20Icon) "(X=20.000000,Y=35.000000)"))
      (bind _questref (Default|GetQuest (Variables|Default|GetAs%20BP%20Game%20Instance) (Variables|Default|GetQuestRow))))
    (:Is%20Not%20Valid
      (bind _returnvalue_2 (Game|ConstructObjectfromClass "/Game/Widget/LocalMapDetails.LocalMapDetails_C"))
      (Variables|Default|SetIcon _returnvalue_2)
      (bind _returnvalue_3 (Game|ConstructObjectfromClass "/Game/Widget/LocalMapDetails.LocalMapDetails_C"))
      (Variables|Default|SetMinimap%20Icon _returnvalue_3)))
  (if (not (.Status (Utilities|Struct|BreakQuestInfo _questref)))
    (return _returnvalue (Variables|Default|GetIcon) _givebacksize (Variables|Default|GetIcon%20Info) "/Game/UI_Assets/question_mark_icon.question_mark_icon" _self (Variables|Default|GetMinimap%20Icon) _givebacksize_2 true)
    (else
      (return _returnvalue (Variables|Default|GetIcon) "" "" 0 _self (Variables|Default|GetMinimap%20Icon) "" false))))