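; Server game mode, by its name, that grants PlayFab virtual currency to tracked players, apparently as a test of end-of-match rewards.
; BeginPlay sets PlayFab credentials with a hard-coded secret key, then calls EndGame after a short delay.
; EndGame requests a fixed credit for each AllPlayers entry and prints debug results.
; AddNewPlayer stores controller and PlayFab ID pairs; its duplicate check only breaks the loop, so the add still runs.
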(event Custom|EndGame
  (for _array_element (Variables|Default|GetAllPlayers)
    (|AddUserVirtualCurrency (Utilities|Struct|MakeAdminAddUserVirtualCurrencyRequest 100 0 (.playerid _array_element) "CR" 0) (delegate Custom|OnAddCurrency) (delegate Custom|Fail))))

(event Custom|OnAddCurrency
  (params (result :type Admin%20Modify%20User%20Virtual%20Currency%20Result%20Structure) (customData :type Object%20Object%20Reference))
  (Development|PrintString "lol"))

(event Custom|Fail
  (params (error :type Play%20Fab%20Error%20Structure) (customData :type Object%20Object%20Reference))
  (Development|PrintString (.errormessage error))
  (Development|PrintString "ggggg"))

(event EventBeginPlay
  (Class|PlayFabUtilities|SetPlayFabSettings "8037B" "FY8Q7PMX43FYPHN3BGOXWHZY4RKGSCRZTSR4JZHBQZ5KM9O9SG")
  (Utilities|FlowControl|Delay 2.0)
  (CallFunction|EndGame))

(event EventTick
  (params (DeltaSeconds :type Float%20%28single-precision%29)))

(fn ConstructionScript)

(fn AddNewPlayer
  (params (PC :type PC%20Object%20Reference) (PlayerID :type String))
  (bind _allplayers (Variables|Default|GetAllPlayers))
  (bind _array_element (Utilities|Array|ForEachLoopwithBreak _allplayers :!label _label)
    (:LoopBody
      (if (or (== PC (.refplayercontroller _array_element)) (Utilities|Enum|Equal(Enum) PlayerID (.playerid _array_element)))
        (goto _label Break)))
    (:Completed
      (Utilities|Array|Add _allplayers (Utilities|Struct|MakePlayerServerData PC PlayerID)))))